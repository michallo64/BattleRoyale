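; BP_Weapon is a weapon Blueprint that tracks clip and spare ammo for its owning BRCharacter.
; On authority, BeginPlay fills the ammo counts and caches the owner, and OnFired decrements the clip, calling Reload when it empties.
; Reload flags the owner as reloading, waits on a fixed delay, then refills from spare ammo.
; HasAmmo reports whether rounds remain; GiveAmmo is empty, with its top-up logic left disconnected.
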(event Custom|Give%20Ammo
  (params (Ammo%20To%20Give :type Integer))
  ;[1 1 1] Event to Give a Weapon ammo
)

(event Custom|On%20Fired
  (bind _currentammo (Variables|Ammo|GetCurrentAmmo))
  (Networking|SwitchHasAuthority
    (:Authority
      (Math|Integer|DecrementInt _currentammo
        (:%20%20
          (if (<= _currentammo 0)
            (CallFunction|Reload)))))))

(event Custom|Reload
  (Variables|/Game/FirstPersonBP/Blueprints/BRCharacter.BRCharacter_C|SetReloading? (Variables|Default|GetAs%20CurrentOwner) true)
  (Utilities|FlowControl|Delay 2.0)
  (Variables|Ammo|SetCurrentAmmo (Math|Integer|Min(Integer) (Variables|Ammo|GetCurrentSpareAmmo) (Variables|Ammo|GetClipSize)))
  (Variables|Ammo|SetCurrentSpareAmmo (Math|Integer|Max(Integer) (- (Variables|Ammo|GetCurrentSpareAmmo) (Math|Integer|Min(Integer) (Variables|Ammo|GetCurrentSpareAmmo) (Variables|Ammo|GetClipSize)))))
  (Variables|/Game/FirstPersonBP/Blueprints/BRCharacter.BRCharacter_C|SetReloading? (Variables|Default|GetAs%20CurrentOwner) false))

(event EventBeginPlay
  ;[1 1 1] On Begin Play set all ammos
  (Networking|SwitchHasAuthority
    (:Authority
      (Variables|Ammo|SetCurrentAmmo (Variables|Ammo|GetClipSize))
      (Variables|Ammo|SetCurrentSpareAmmo (Variables|Ammo|GetStartingSpareAmmo))
      (bind _asbrcharacter (Utilities|Casting|CastToBRCharacter (Components|GetOwner)))
      (Variables|Default|SetAs%20CurrentOwner _asbrcharacter))))

(fn ConstructionScript)

(fn HasAmmo?
  (return (> (Variables|Ammo|GetCurrentAmmo) 0)))