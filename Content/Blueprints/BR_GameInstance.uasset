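; BR_GameInstance is a Game Instance Blueprint that gets the player into a multiplayer session, either joining or hosting one.
; TryJoinOrCreateGame searches for sessions, optionally over LAN, and passes the first result to JoinBPSession.
; If the search is empty or fails, it creates a session and opens FirstPersonExampleMap as a listen server.
; Successful joining or hosting switches to game-only input without a cursor; failures only print an error.
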(event Custom|Try%20Join%20Or%20Create%20Game
  (bind _returnvalue (Game|GetPlayerController 0))
  ;[1 1 1] Try Join or Create session
  (bind _results (|FindSessions (Game|GetPlayerController 0) 20 (Variables|Default|GetUse%20LAN?))
    (:OnSuccess
      (if (Utilities|Array|IsValidIndex _results)
        (CallFunction|JoinBPSession (Utilities|Array|Get(acopy) _results))
        (else
          (|Session (Game|GetPlayerController 0) 20 (Variables|Default|GetUse%20LAN?) :!label _label
            (:OnSuccess
              (Game|OpenLevel(byName) "FirstPersonExampleMap" true "listen")
              (Variables|/Script/Engine.PlayerController|SetbShowMouseCursor _returnvalue false)
              (Input|SetInputModeGameOnly _returnvalue))
            (:OnFailure
              (Development|PrintString "ERROR CREATING SESSION"))))))
    (:OnFailure
      (goto _label))))

(event Custom|Join%20BP%20Session
  (params (Session :type Blueprint%20Session%20Result%20Structure))
  (bind _returnvalue (Game|GetPlayerController 0))
  ;[1 1 1] Join a Session
  (|JoinSession (Game|GetPlayerController 0) Session
    (:OnSuccess
      (Variables|/Script/Engine.PlayerController|SetbShowMouseCursor _returnvalue false)
      (Input|SetInputModeGameOnly _returnvalue))
    (:OnFailure
      (Development|PrintString "ERROR JOINING SESSION"))))